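; BP_Enemy is an AI enemy character that spawns with an assault rifle and a pistol and manages its own weapon choice.
; ArmSelf keeps the held gun while it has loaded or reserve ammo, otherwise equips the first usable weapon or unequips.
; CheckAmmo reports whether the held gun is empty and can reload.
; The ChangeGunInHand override updates the blackboard's IsArmed key on authority only.
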(event Custom|ArmSelf
  (bind _returnvalue (CallFunction|IsUsableWeapon (Variables|Default|GetGunInHand)))
  (if (not _returnvalue)
    (bind _slot (CallFunction|FindUsableWeapon))
    (if (>= _slot 0)
      (CallFunction|Equip _slot)
      (else
        (CallFunction|Unequip)))))

(event EventBeginPlay
  (|CallParentFunction)
  (bind _returnvalue (Game|SpawnActorfromClass "/Game/Blueprints/Weapon/Gun/BP_Gun_AssaultRifle.BP_Gun_AssaultRifle_C" (Math|Transform|MakeTransform "0, 0, 0") "AdjustIfPossibleButAlwaysSpawn" 0 0))
  (CallFunction|ClientGetGun _returnvalue)
  (bind _returnvalue_2 (Game|SpawnActorfromClass "/Game/Blueprints/Weapon/Gun/BP_Gun_Pistol.BP_Gun_Pistol_C" (Math|Transform|MakeTransform "0, 0, 0") "AdjustIfPossibleButAlwaysSpawn" 0 0))
  (CallFunction|ClientGetGun _returnvalue_2))

(fn ConstructionScript
  (|CallParentFunction))

(fn IsUsableWeapon
  (params (Weapon :type BPM%20Gun%20Object%20Reference))
  (Utilities|IsValid Weapon
    (:Is%20Valid
      (bind _curammo (Default|GetCurrentAmmo Weapon))
      (return (or (> _curammo 0) (> (CallFunction|GetRemainAmmo (Variables|/Game/Blueprints/Weapon/Gun/BPM_Gun.BPM_Gun_C|GetGunType Weapon)) 0))))
    (:Is%20Not%20Valid
      (return false))))

(fn CheckAmmo
  (if (Utilities|Enum|NotEqual(Enum) (Variables|Default|GetArmedType) "NewEnumerator0")
    (bind _curammo (Default|GetCurrentAmmo (Variables|Default|GetGunInHand)))
    (if (> _curammo 0)
      (return false false)
      (else
        (return true (> (CallFunction|GetRemainAmmo (Variables|Default|GetArmedType)) 0))))
    (else
      (return false false))))

(fn ChangeGuninHand
  (params (Slot :type Integer))
  (|CallParentFunction Slot)
  (Networking|SwitchHasAuthority
    (:Authority
      (if (>= Slot 0)
        (AI|Components|Blackboard|SetValueasBool (AI|GetBlackboard 0) (Utilities|Name|MakeLiteralName "IsArmed") true)
        (else
          (AI|Components|Blackboard|SetValueasBool (AI|GetBlackboard 0) (Utilities|Name|MakeLiteralName "IsArmed") false))))))

(fn FindUsableWeapon
  (bind (_array_element _array_index) (Utilities|Array|ForEachLoopwithBreak (Variables|Default|GetWeapons))
    (:LoopBody
      (bind _returnvalue (CallFunction|IsUsableWeapon _array_element))
      (if _returnvalue
        (return _array_index)))
    (:Completed
      (return -1))))