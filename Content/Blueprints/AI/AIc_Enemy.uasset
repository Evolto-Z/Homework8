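; AI controller for enemies that runs the BT_Enemy behavior tree and feeds its Blackboard from sight and hearing perception.
; The first sighted actor becomes the focused Enemy target and is held until sight of it is lost.
; Lost sightings and heard stimuli record their position as EnemyLocation.
; Any detection sets IsVigilant, which this controller never clears.
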(event OnTargetPerceptionUpdated(Sight)
  (params (Actor :type Actor%20Object%20Reference) (Stimulus :type AI%20Stimulus%20Structure))
  (bind (_age _expirationage _strength _stimuluslocation _receiverlocation _tag _bsuccessfullysensed) (Utilities|Struct|BreakAIStimulus Stimulus))
  (if _bsuccessfullysensed
    (Utilities|IsValid (Variables|Default|GetTargetActor)
      (:Is%20Not%20Valid
        (CallFunction|FindTargetActor Actor)))
    (else
      (CallFunction|NoticeTargetLocation _stimuluslocation)
      (if (== Actor (Variables|Default|GetTargetActor))
        (CallFunction|LoseTargetActor)))))

(event OnTargetPerceptionUpdated(Hearing)
  (params (Actor :type Actor%20Object%20Reference) (Stimulus :type AI%20Stimulus%20Structure))
  (bind (_age _expirationage _strength _stimuluslocation _receiverlocation _tag _bsuccessfullysensed) (Utilities|Struct|BreakAIStimulus Stimulus))
  (if _bsuccessfullysensed
    (CallFunction|NoticeTargetLocation _stimuluslocation)))

(event EventBeginPlay
  (AI|RunBehaviorTree "/Game/Blueprints/AI/BT_Enemy.BT_Enemy"))

(fn ConstructionScript)

(fn FindTargetActor
  (params (Actor :type Actor%20Object%20Reference%20%28by%20ref%29))
  (bind _output_get (Variables|Default|SetTargetActor Actor))
  (AI|SetFocus _output_get)
  (AI|Components|Blackboard|SetValueasObject (Variables|Default|GetBlackboard) (Utilities|Name|MakeLiteralName "Enemy") _output_get)
  (AI|Components|Blackboard|SetValueasBool (Variables|Default|GetBlackboard) (Utilities|Name|MakeLiteralName "IsVigilant") true))

(fn LoseTargetActor
  (Variables|Default|SetTargetActor 0)
  (AI|ClearFocus)
  (AI|Components|Blackboard|SetValueasObject (Variables|Default|GetBlackboard) (Utilities|Name|MakeLiteralName "Enemy") 0))

(fn NoticeTargetLocation
  (params (Location :type Vector%20%28by%20ref%29))
  (AI|Components|Blackboard|SetValueasVector (Variables|Default|GetBlackboard) (Utilities|Name|MakeLiteralName "EnemyLocation") Location)
  (AI|Components|Blackboard|SetValueasBool (Variables|Default|GetBlackboard) (Utilities|Name|MakeLiteralName "IsVigilant") true))