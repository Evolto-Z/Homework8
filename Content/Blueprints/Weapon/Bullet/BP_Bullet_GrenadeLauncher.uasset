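; Grenade launcher bullet that explodes on hit, dealing radial damage and a physics impulse.
; On hit it spawns explosion effects at the impact point, and only the server applies damage and fires the impulse before the actor is destroyed.
; Radial damage can skip the instigator, and the construction script matches the radial force radius to the damage radius.
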(event Collision|EventHit
  (params (MyComp :type Primitive%20Component%20Object%20Reference) (Other :type Actor%20Object%20Reference) (OtherComp :type Primitive%20Component%20Object%20Reference) (bSelfMoved :type Boolean) (HitLocation :type Vector :default "0, 0, 0") (HitNormal :type Vector :default "0, 0, 0") (NormalImpulse :type Vector :default "0, 0, 0") (Hit :type Hit%20Result%20Structure%20%28by%20ref%29))
  ;[1 1 1] On Hit
  (CallFunction|GenerateEffects HitLocation HitNormal OtherComp "/Game/MilitaryWeapSilver/FX/P_Grenade_Explosion_01.P_Grenade_Explosion_01")
  (if (Networking|IsServer)
    (|CauseDamage)
    (|CauseImpulse)
    (Actor|DestroyActor)
    (else
      (Actor|DestroyActor))))

(fn ConstructionScript
  (|CallParentFunction)
  (Variables|/Script/Engine.RadialForceComponent|SetRadius (Variables|Default|GetRadialForce) (Variables|Default|GetDamageRadius)))